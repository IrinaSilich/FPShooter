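; BP_BotParent is a parent AI bot that shoots at its controller's focus actor, takes damage and dies.
; Shooting traces from the gun toward a randomly rotated target location for spread, applying point damage with sound and muzzle flash.
; Non-lethal point and radial hits report damage events for AI sensing.
; Point death plays a montage, then swaps in a static corpse mesh; radial death ragdolls, and both unpossess and expire.
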(event Custom|Shooting
  (bind _self self)
  (bind _gun (Variables|Default|GetGun))
  (bind _returnvalue (AI|GetAIController _self))
  (bind _returnvalue_2 (Class|AIController|GetFocusActor _returnvalue))
  ;[1 1 1] Checking Focus Actor
  (Utilities|IsValid _returnvalue_2
    (:Is%20Valid
      ;[1 1 1] Line Trace
      (bind _outhit (Collision|LineTraceByChannel (Transformation|GetWorldLocation (Variables|Default|GetGun)) (Math|Vector|RotateVector (Transformation|GetActorLocation _returnvalue_2) (Math|Rotator|MakeRotator (Math|Random|RandomFloatinRange -0.09 0.09) 0.0 (Math|Random|RandomFloatinRange -0.09 0.09))) "TraceTypeQuery1" false 0 "None"))
      ;[1 1 1] Applying Damage
      (Game|Damage|ApplyPointDamage (.HitActor (Collision|BreakHitResult _outhit)) (Variables|Default|GetDamageAmount) (.ImpactNormal (Collision|BreakHitResult _outhit)) _outhit 0 self)
      ;[1 1 1] Playing Shot Sound
      (Audio|PlaySoundatLocation "/Game/Assets/Effects/SFX/GunShotCue.GunShotCue" (Transformation|GetActorLocation) "0, 0, 0" 0.5 1.0 0.0 0 0 0)
      ;[1 1 1] Spawning Muzzle Flash
      (bind _returnvalue_3 (Effects|SpawnEmitteratLocation "/Game/Assets/Effects/VFX/Weapon/ParticleSystems/Weapons/AssaultRifle/Muzzle/P_AssaultRifle_MF.P_AssaultRifle_MF" (Transformation|GetSocketLocation _gun "MuzzleFlashSocket") (Transformation|GetSocketRotation _gun "MuzzleFlashSocket")))
      (Utilities|FlowControl|Delay 0.1)
      (Components|DestroyComponent _returnvalue_3))))

(event Custom|PointDeath
  (bind _mesh (Variables|Character|GetMesh))
  (bind _mesh_2 (Variables|Character|GetMesh))
  (bind _corpse (Variables|Default|GetCorpse))
  ;[1 1 1] Death From Point Damage
  (Animation|Montage|PlayMontage _mesh_2 "/Game/Assets/Bot/Animations/Death_1_Montage.Death_1_Montage"
    (:then
      (Pawn|UnPossess (AI|GetAIController self))
      (Collision|SetCollisionEnabled _mesh_2 "NoCollision")
      (Collision|SetCollisionEnabled (Variables|Collision|GetCapsuleComponent) "NoCollision")
      (Actor|SetLifeSpan 5.0))
    (:OnBlendOut
      ;[1 1 1] Setting Corpse
      (Components|StaticMesh|SetStaticMesh (Variables|Default|GetCorpse) "/Game/Assets/Bot/Mesh/SM_Death.SM_Death")
      (Transformation|SetWorldRotation _corpse (Transformation|GetWorldRotation _mesh) false false)
      (Transformation|SetWorldLocation _corpse (Transformation|GetWorldLocation _mesh) false false)
      (Components|DestroyComponent (Variables|Character|GetMesh))
      (Rendering|SetVisibility (Variables|Default|GetCorpse) true false))))

(event Custom|RadialDeath
  ;[1 1 1] Death From Radial Damage
  (Pawn|UnPossess (AI|GetAIController self))
  (Collision|SetCollisionEnabled (Variables|Character|GetMesh) "PhysicsOnly")
  (Collision|SetCollisionEnabled (Variables|Collision|GetCapsuleComponent) "PhysicsOnly")
  (Physics|SetSimulatePhysics (Variables|Character|GetMesh) true)
  (Actor|SetLifeSpan 5.0))

(event Game|Damage|EventPointDamage
  (params (Damage :type Float%20%28single-precision%29) (DamageType :type Damage%20Type%20Object%20Reference) (HitLocation :type Vector :default "0, 0, 0") (HitNormal :type Vector :default "0, 0, 0") (HitComponent :type Primitive%20Component%20Object%20Reference) (BoneName :type Name :default "None") (ShotFromDirection :type Vector :default "0, 0, 0") (InstigatedBy :type Controller%20Object%20Reference) (DamageCauser :type Actor%20Object%20Reference) (HitInfo :type Hit%20Result%20Structure%20%28by%20ref%29))
  ;[1 1 1] Taking Point Damage
  (bind _output_get (Variables|Default|SetHealthCurrent (Math|Float|Max(Float) (- (Variables|Default|GetHealthCurrent) Damage) 0.0)))
  (if (Math|Float|NearlyEqual(Float) _output_get 0.0 1e-06)
    (CallFunction|PointDeath)
    (else
      (Class|AISenseDamage|ReportDamageEvent self DamageCauser Damage (Transformation|GetActorLocation) "0, 0, 0" "None"))))

(event EventBeginPlay
  (Rendering|SetVisibility (Variables|Default|GetCorpse) false false))

(event Game|Damage|EventRadialDamage
  (params (DamageReceived :type Float%20%28single-precision%29) (DamageType :type Damage%20Type%20Object%20Reference) (Origin :type Vector :default "0, 0, 0") (HitInfo :type Hit%20Result%20Structure%20%28by%20ref%29) (InstigatedBy :type Controller%20Object%20Reference) (DamageCauser :type Actor%20Object%20Reference))
  ;[1 1 1] Taking Radial Damage
  (bind _output_get (Variables|Default|SetHealthCurrent (Math|Float|Max(Float) (- (Variables|Default|GetHealthCurrent) DamageReceived) 0.0)))
  (if (Math|Float|NearlyEqual(Float) _output_get 0.0 1e-06)
    (CallFunction|RadialDeath)
    (else
      (Class|AISenseDamage|ReportDamageEvent self DamageCauser DamageReceived (Transformation|GetActorLocation) "0, 0, 0" "None"))))

(fn ConstructionScript
  (GameplayTags|AddGameplayTag (Variables|Default|GetTagContainer) (Variables|Default|GetTeamTag) :!class /Script/GameplayTags.BlueprintGameplayTagLibrary))