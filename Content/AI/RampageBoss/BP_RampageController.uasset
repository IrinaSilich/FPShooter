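; AI controller for the Rampage boss that starts its behavior tree and relays attack commands to the boss character.
; On BeginPlay it async-loads the behavior tree, runs it, then caches the player character and the controlled Rampage character.
; Its Attack event forwards to the cached Rampage character's Attack.
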(event Custom|Attack
  (Default|Attack (Variables|Default|GetRampageCharacter)))

(event EventBeginPlay
  (bind _object (Utilities|AsyncLoadAsset (Variables|Default|GetBehaviourTree))
    (:Completed
      (bind _asbehavior_tree (Utilities|Casting|CastToBehaviorTree _object))
      (AI|RunBehaviorTree _asbehavior_tree)
      (bind _asbp_player_character (Utilities|Casting|CastToBP_PlayerCharacter (Game|GetPlayerCharacter 0)))
      (Variables|Default|SetPlayerCharacter _asbp_player_character)
      (bind _asbp_rampage_character (Utilities|Casting|CastToBP_RampageCharacter (Pawn|GetControlledPawn)))
      (Variables|Default|SetRampageCharacter _asbp_rampage_character))))

(fn ConstructionScript)