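; BP_GameMode is the level's game mode, handling background music and player respawn.
; A Music component starts on BeginPlay, and the ChangeMusic event swaps it to the MeetingRampage track and restarts it.
; RespawnCharacter continues only if player 0's character is a BP_PlayerCharacter, waits RespawnDelay, then spawns the Character class at SpawnTransform and has the player controller possess it.
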(event Custom|RespawnCharacter
  ;[1 1 1] Player Respawn
  (Utilities|Casting|CastToBP_PlayerCharacter (Game|GetPlayerCharacter 0))
  (Utilities|FlowControl|Delay (Variables|Default|GetRespawnDelay))
  (bind _returnvalue (Game|SpawnActorfromClass (Variables|Default|GetCharacter) (Variables|Default|GetSpawnTransform) "Undefined" 0 0))
  (Pawn|Possess (Game|GetPlayerController 0) _returnvalue))

(event Custom|ChangeMusic
  (bind _music (Variables|Default|GetMusic))
  ;[1 1 1] Setting Rampage Music
  (Audio|Components|Audio|SetSound _music "/Game/Assets/Effects/SFX/MeetingRampage.MeetingRampage")
  (Audio|Components|Audio|Play _music 0.0))

(event EventBeginPlay
  ;[1 1 1] Setting Main Music
  (Audio|Components|Audio|Play (Variables|Default|GetMusic) 0.0))

(fn ConstructionScript)